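; Player character for a speaker who moves along the view direction and steps through presentation slides.
; Slide inputs change CurrentSlide, floored at one only when going back, and notify ScreenBP actors.
; A received room code is stored and forwarded to the StartMenu widget, while pausing shows a PauseMenu.
; Right mouse and motion-controller face buttons simulate widget left clicks, the latter only in MainMenu or when paused.
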(event Custom|Set%20Room%20Code
  (params (code :type String))
  ;[1 1 1] Set room code
  (bind _output_get (Variables|Default|SetRoom%20Code code))
  (bind _foundwidgets (Widget|GetAllWidgetsOfClass "/Game/UI/StartMenu.StartMenu_C" true))
  (bind _asstart_menu (Utilities|Casting|CastToStartMenu (Utilities|Array|Get(acopy) _foundwidgets)))
  (Default|RoomCodeRecieved _asstart_menu _output_get))

(event EventBeginPlay
  (Variables|Default|SetcurrentSlide 1))

(event Collision|EventActorBeginOverlap
  (params (OtherActor :type Actor%20Object%20Reference)))

(event EventTick
  (params (DeltaSeconds :type Float%20%28single-precision%29)))

(event Input|ActionEvents|InputActionpause
  (params (Key :type Key%20Structure))
  ;[1 1 1] Pause game
  (:Pressed
    (CallFunction|PauseGame)))

(event Input|ActionEvents|InputActionnextSlide
  (params (Key :type Key%20Structure))
  ;[1 1 1] Next Slide
  (:Pressed
    (Development|PrintString "Next slide")
    (bind _result (Math|Integer|IncrementInt (Variables|Default|GetcurrentSlide))
      (:%20%20
        (Variables|Default|SetcurrentSlide _result)
        (bind _outactors (Actor|GetAllActorsOfClass "/Game/Blueprints/ScreenBP.ScreenBP_C"))
        (Default|SlideDidChange _outactors)))))

(event Input|ActionEvents|InputActionprevSlide
  (params (Key :type Key%20Structure))
  ;[1 1 1] Previous Slide
  (:Pressed
    (Development|PrintString "Previous Slide")
    (if (not (== 1 (Variables|Default|GetcurrentSlide)))
      (bind _result (Math|Integer|DecrementInt (Variables|Default|GetcurrentSlide))
        (:%20%20
          (Variables|Default|SetcurrentSlide _result)
          (bind _outactors (Actor|GetAllActorsOfClass "/Game/Blueprints/ScreenBP.ScreenBP_C"))
          (Default|SlideDidChange _outactors))))))

(event Input|AxisEvents|InputAxisforward
  (params (AxisValue :type Float%20%28single-precision%29))
  ;[1 1 1] Move Forward
  (Pawn|Input|AddMovementInput (Math|Vector|GetForwardVector (Pawn|GetControlRotation :!class /Script/Engine.Pawn)) AxisValue false))

(event Input|AxisEvents|InputAxisbackward
  (params (AxisValue :type Float%20%28single-precision%29))
  ;[1 1 1] Move Backwards
  (Pawn|Input|AddMovementInput (Math|Vector|GetForwardVector (Pawn|GetControlRotation :!class /Script/Engine.Pawn)) AxisValue false))

(event Input|MouseEvents|RightMouseButton
  (params (Key :type Key%20Structure))
  (bind _widgetinteraction (Variables|Default|GetWidgetInteraction))
  (:Pressed
    (Class|WidgetInteractionComponent|PressPointerKey _widgetinteraction "LeftMouseButton"))
  (:Released
    (Class|WidgetInteractionComponent|ReleasePointerKey _widgetinteraction "LeftMouseButton")))

(event Input|KeyboardEvents|MotionControllerRightFaceButton1
  (params (Key :type Key%20Structure))
  (bind _widgetinteraction (Variables|Default|GetWidgetInteraction))
  (:Pressed
    (bind _returnvalue (Game|GetCurrentLevelName true))
    (if (or (Utilities|Enum|Equal(Enum) _returnvalue "MainMenu") (Variables|Default|GetPaused))
      (Class|WidgetInteractionComponent|PressPointerKey _widgetinteraction "LeftMouseButton")))
  (:Released
    (bind _returnvalue_2 (Game|GetCurrentLevelName true))
    (if (or (Utilities|Enum|Equal(Enum) _returnvalue_2 "MainMenu") (Variables|Default|GetPaused))
      (Class|WidgetInteractionComponent|ReleasePointerKey _widgetinteraction "LeftMouseButton"))))

(event Input|KeyboardEvents|MotionControllerLeftFaceButton1
  (params (Key :type Key%20Structure))
  (bind _widgetinteraction (Variables|Default|GetWidgetInteraction))
  (:Pressed
    (bind _returnvalue (Game|GetCurrentLevelName true))
    (if (or (Utilities|Enum|Equal(Enum) _returnvalue "MainMenu") (Variables|Default|GetPaused))
      (Class|WidgetInteractionComponent|PressPointerKey _widgetinteraction "LeftMouseButton")))
  (:Released
    (bind _returnvalue_2 (Game|GetCurrentLevelName true))
    (if (or (Utilities|Enum|Equal(Enum) _returnvalue_2 "MainMenu") (Variables|Default|GetPaused))
      (Class|WidgetInteractionComponent|ReleasePointerKey _widgetinteraction "LeftMouseButton"))))

(fn ConstructionScript)

(fn PauseGame
  (Game|SetGamePaused true)
  (Utilities|IsValid 0
    (:Is%20Valid
      _)
    (:Is%20Not%20Valid
      (bind _returnvalue (UserInterface|CreateWidget "/Game/UI/PauseMenu.PauseMenu_C" (Game|GetPlayerController 0)))
      (Variables|Default|SetPause%20Menu _returnvalue)))
  (UserInterface|Viewport|AddtoViewport (Variables|Default|GetPause%20Menu) 0)
  (Input|SetInputModeUIOnly 0 (Variables|Default|GetPause%20Menu) "DoNotLock"))

(fn UnpauseGame
  (Game|SetGamePaused false)
  (Viewport|RemoveAllWidgets)
  (Input|SetInputModeGameOnly (Game|GetPlayerController 0)))