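; Presentation screen actor that displays the current slide of the speaker's room on its Cube mesh.
; RoomDidLoad and SlideDidChange read RoomCode and CurrentSlide from player 0's SpeakerPlayerCharacter and download that slide image from a hardcoded HTTP server.
; On success, each applies the image as the Texture parameter of a new dynamic ScreenMaterial instance.
; The SetSlide function is unfinished, with its download and apply logic disconnected.
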(event Custom|Slide%20Did%20Change
  (bind _asspeaker_player_character (Utilities|Casting|CastToSpeakerPlayerCharacter (Game|Player|GetPlayerPawn 0)))
  (bind _texture (|DownloadImage (Utilities|String|Append "http://104.131.9.190:3000/r/" (Variables|/Game/Blueprints/SpeakerPlayerCharacter.SpeakerPlayerCharacter_C|GetRoom%20Code _asspeaker_player_character) "/slides?index=" (Utilities|String|ToString(Integer) (Variables|/Game/Blueprints/SpeakerPlayerCharacter.SpeakerPlayerCharacter_C|GetcurrentSlide _asspeaker_player_character))))
    (:OnSuccess
      (bind _returnvalue (Rendering|Material|CreateDynamicMaterialInstance "/Game/Blueprints/ScreenMaterial.ScreenMaterial" :!class /Script/Engine.KismetMaterialLibrary))
      (Rendering|Material|SetTextureParameterValue _returnvalue "Texture" _texture)
      (Rendering|Material|SetMaterial (Variables|Default|GetCube) 0 _returnvalue))))

(event Custom|Room%20Did%20Load
  (bind _asspeaker_player_character (Utilities|Casting|CastToSpeakerPlayerCharacter (Game|Player|GetPlayerPawn 0)))
  (bind _texture (|DownloadImage (Utilities|String|Append "http://104.131.9.190:3000/r/" (Variables|/Game/Blueprints/SpeakerPlayerCharacter.SpeakerPlayerCharacter_C|GetRoom%20Code _asspeaker_player_character) "/slides?index=" (Utilities|String|ToString(Integer) (Variables|/Game/Blueprints/SpeakerPlayerCharacter.SpeakerPlayerCharacter_C|GetcurrentSlide _asspeaker_player_character))))
    (:OnSuccess
      (bind _returnvalue (Rendering|Material|CreateDynamicMaterialInstance "/Game/Blueprints/ScreenMaterial.ScreenMaterial" :!class /Script/Engine.KismetMaterialLibrary))
      (Rendering|Material|SetTextureParameterValue _returnvalue "Texture" _texture)
      (Rendering|Material|SetMaterial (Variables|Default|GetCube) 0 _returnvalue))))

(event EventBeginPlay)

(event Collision|EventActorBeginOverlap
  (params (OtherActor :type Actor%20Object%20Reference)))

(event EventTick
  (params (DeltaSeconds :type Float%20%28single-precision%29)))

(fn ConstructionScript)

(fn SetSlide
  (bind _asspeaker_player_character (Utilities|Casting|CastToSpeakerPlayerCharacter (Game|Player|GetPlayerPawn 0)))
  (bind _returnvalue (Rendering|Material|CreateDynamicMaterialInstance "/Game/Blueprints/ScreenMaterial.ScreenMaterial" :!class /Script/Engine.KismetMaterialLibrary)))