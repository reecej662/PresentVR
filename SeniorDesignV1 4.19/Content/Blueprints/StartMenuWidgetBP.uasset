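; StartMenuWidgetBP is a Blueprint that hosts the StartMenu UI in a Widget component and relays the room code to it.
; On RoomCodeReceived, it reads RoomCode from the SpeakerPlayerCharacter pawn of player 0 and passes it to the StartMenu widget, stopping if either cast fails.
; An unreached fragment would swap in a Summary widget, and the other events and construction script are empty.
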(event Custom|Room%20Code%20Received
  (bind _asspeaker_player_character (Utilities|Casting|CastToSpeakerPlayerCharacter (Game|Player|GetPlayerPawn 0)))
  (bind _asstart_menu (Utilities|Casting|CastToStartMenu (UserInterface|GetUserWidgetObject (Variables|Default|GetWidget))))
  (Default|RoomCodeRecieved _asstart_menu (Variables|/Game/Blueprints/SpeakerPlayerCharacter.SpeakerPlayerCharacter_C|GetRoom%20Code _asspeaker_player_character)))

(event EventBeginPlay)

(event Collision|EventActorBeginOverlap
  (params (OtherActor :type Actor%20Object%20Reference)))

(event EventTick
  (params (DeltaSeconds :type Float%20%28single-precision%29)))

(fn ConstructionScript)