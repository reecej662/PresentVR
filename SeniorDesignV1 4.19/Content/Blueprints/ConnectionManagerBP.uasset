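; Actor that relays Socket.IO server events into a speaking scene with an audience, a screen and the speaker player.
; It binds named events on BeginPlay and routes each by name to the speaker character, ScreenBP or AudiencePawns.
; Interest, mood and action apply to every audience pawn, while emotion messages reach only the first.
; A transcript event requests the opening words back over the socket and shows the notecard.
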(event OnEvent(SocketIOClient)
  (params (Event :type String) (MessageJson :type SIO%20Json%20Value%20Object%20Reference))
  (bind _returnvalue (Class|SIOJsonValue|AsString MessageJson))
  (bind _returnvalue_2 (Game|Player|GetPlayerPawn 0))
  (bind _returnvalue_3 (Math|Conversions|ToInteger(Byte) _returnvalue))
  ;[1 1 1] Socket event happens
  (if (Utilities|Enum|Equal(Enum) Event "new message")
    (bind _outactors (Actor|GetAllActorsOfClass "/Game/Blueprints/AudiencePawn.AudiencePawn_C"))
    (bind _asaudience_pawn (Utilities|Casting|CastToAudiencePawn (Utilities|Array|Get(acopy) _outactors)))
    (Default|EmotionUpdate _asaudience_pawn _returnvalue)
    (elif (Utilities|Enum|Equal(Enum) Event "room code")
      (bind _asspeaker_player_character (Utilities|Casting|CastToSpeakerPlayerCharacter (Game|GetPlayerCharacter 0)))
      (Default|SetRoomCode _asspeaker_player_character _returnvalue)
      (bind _outactors_2 (Actor|GetAllActorsOfClass "/Game/Blueprints/ScreenBP.ScreenBP_C"))
      (Default|RoomDidLoad (Utilities|Array|Get(acopy) _outactors_2))
      (elif (Utilities|Enum|Equal(Enum) Event "presentation")
        (bind _outactors_3 (Actor|GetAllActorsOfClass "/Game/Blueprints/ScreenBP.ScreenBP_C"))
        (Default|RoomDidLoad (Utilities|Array|Get(acopy) _outactors_3))
        (elif (Utilities|Enum|Equal(Enum) Event "transcriptUpdate")
          (bind _asspeaker_player_character_2 (Utilities|Casting|CastToSpeakerPlayerCharacter _returnvalue_2))
          (Default|UpdateTranscript _asspeaker_player_character_2 _returnvalue)
          (elif (Utilities|Enum|Equal(Enum) Event "transcript")
            (CallFunction|RequestTranscript 0 5)
            (bind _asspeaker_player_character_3 (Utilities|Casting|CastToSpeakerPlayerCharacter _returnvalue_2))
            (Default|ShowNotecard _asspeaker_player_character_3)
            (elif (Utilities|Enum|Equal(Enum) Event "interest")
              (bind _outactors_4 (Actor|GetAllActorsOfClass "/Game/Blueprints/AudiencePawn.AudiencePawn_C"))
              (for _array_element _outactors_4
                (Variables|/Game/Blueprints/AudiencePawn.AudiencePawn_C|Setinterest _array_element _returnvalue_3))
              (elif (Utilities|Enum|Equal(Enum) Event "mood")
                (bind _outactors_5 (Actor|GetAllActorsOfClass "/Game/Blueprints/AudiencePawn.AudiencePawn_C"))
                (for _array_element_2 _outactors_5
                  (Variables|/Game/Blueprints/AudiencePawn.AudiencePawn_C|Setmood _array_element_2 _returnvalue_3))
                (elif (Utilities|Enum|Equal(Enum) Event "action")
                  (bind _outactors_6 (Actor|GetAllActorsOfClass "/Game/Blueprints/AudiencePawn.AudiencePawn_C"))
                  (for _array_element_3 _outactors_6
                    (Default|UpdateAction _array_element_3 _returnvalue_3)))))))))))

(event OnConnected(SocketIOClient)
  (params (SessionId :type String) (bIsReconnection :type Boolean))
  ;[1 1 1] Socket is connected
  (Development|PrintString "Connected"))

(event OnDisconnected(SocketIOClient)
  (params (Reason :type ESIOConnectionCloseReason%20Enum :default "CLOSE_REASON_NORMAL"))
  ;[1 1 1] Socket is disconnected
  (Development|PrintString (Utilities|String|Append "Disconnected" (Utilities|String|EnumtoString Reason))))

(event EventBeginPlay
  (bind _socketioclient (Variables|Default|GetSocketIOClient))
  ;[1 1 1] Binds event 'new message' to the socket client
  (Class|SocketIOClientComponent|BindEvent _socketioclient "new message" "/")
  (Class|SocketIOClientComponent|BindEvent _socketioclient "room code" "/")
  (Class|SocketIOClientComponent|BindEvent _socketioclient "presentation" "/")
  (Class|SocketIOClientComponent|BindEvent _socketioclient "transcriptUpdate" "/")
  (Class|SocketIOClientComponent|BindEvent _socketioclient "transcript" "/")
  (Class|SocketIOClientComponent|BindEvent _socketioclient "interest" "/")
  (Class|SocketIOClientComponent|BindEvent _socketioclient "mood" "/")
  (Class|SocketIOClientComponent|BindEvent _socketioclient "action" "/"))

(event Collision|EventActorBeginOverlap
  (params (OtherActor :type Actor%20Object%20Reference)))

(event EventTick
  (params (DeltaSeconds :type Float%20%28single-precision%29)))

(fn ConstructionScript)

(fn RequestTranscript
  (params (index :type Integer) (words :type Integer))
  (Class|SocketIOClientComponent|Emit (Variables|Default|GetSocketIOClient) "updateTranscript" (Class|SIOJLibrary|ToJsonValue(String) (Utilities|String|Append "{\"index\":" (Utilities|String|ToString(Integer) index) ", \"words\":" (Utilities|String|ToString(Integer) words) "}")) "/"))