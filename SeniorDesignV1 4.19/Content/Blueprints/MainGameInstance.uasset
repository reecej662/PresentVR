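; Game instance that opens the game's UI screens: main menu, classroom selection, summary and pause menu.
; Each event lazily creates and caches its widget, adds it to the viewport and switches to UI-only input with the cursor shown.
; PauseGame never stores its created widget, setting PauseRef to None, and does not pause gameplay.
; ShowConferenceRoomSelect is empty, with its selection-screen logic left disconnected.
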(event Custom|PauseGame
  (bind _returnvalue (Game|GetPlayerController 0))
  (Utilities|IsValid (Variables|Default|GetPauseRef)
    (:Is%20Valid
      _)
    (:Is%20Not%20Valid
      (UserInterface|CreateWidget "/Game/UI/PauseMenu.PauseMenu_C")
      (Variables|Default|SetPauseRef 0)))
  (UserInterface|Viewport|AddtoViewport (Variables|Default|GetPauseRef) 0)
  (Input|SetInputModeUIOnly _returnvalue (Variables|Default|GetPauseRef) "DoNotLock")
  (Variables|/Script/Engine.PlayerController|SetbShowMouseCursor _returnvalue true))

(event Custom|ShowConferenceRoomSelect)

(event Custom|ShowSummary
  (bind _returnvalue (Game|GetPlayerController 0))
  (Utilities|IsValid (Variables|Default|GetSummaryRef)
    (:Is%20Valid
      _)
    (:Is%20Not%20Valid
      (bind _returnvalue_2 (UserInterface|CreateWidget "/Game/Blueprints/summary.summary_C"))
      (Variables|Default|SetSummaryRef _returnvalue_2)))
  (UserInterface|Viewport|AddtoViewport (Variables|Default|GetSummaryRef) 0)
  (Input|SetInputModeUIOnly _returnvalue (Variables|Default|GetSummaryRef) "DoNotLock")
  (Variables|/Script/Engine.PlayerController|SetbShowMouseCursor _returnvalue true))

(event Custom|ShowClassRoomSelect
  (bind _returnvalue (Game|GetPlayerController 0))
  (Utilities|IsValid (Variables|Default|GetClassRoomRef)
    (:Is%20Valid
      _)
    (:Is%20Not%20Valid
      (bind _returnvalue_2 (UserInterface|CreateWidget "/Game/Blueprints/SelectClass.SelectClass_C"))
      (Variables|Default|SetClassRoomRef _returnvalue_2)))
  (UserInterface|Viewport|AddtoViewport (Variables|Default|GetClassRoomRef) 0)
  (Input|SetInputModeUIOnly _returnvalue (Variables|Default|GetClassRoomRef) "DoNotLock")
  (Variables|/Script/Engine.PlayerController|SetbShowMouseCursor _returnvalue true))

(event Custom|ShowMainMenu
  (bind _returnvalue (Game|GetPlayerController 0))
  (Utilities|IsValid (Variables|Default|GetMainMenuRef)
    (:Is%20Valid
      _)
    (:Is%20Not%20Valid
      (bind _returnvalue_2 (UserInterface|CreateWidget "/Game/Blueprints/MainMenu.MainMenu_C"))
      (Variables|Default|SetMainMenuRef _returnvalue_2)))
  (UserInterface|Viewport|AddtoViewport (Variables|Default|GetMainMenuRef) 0)
  (Input|SetInputModeUIOnly _returnvalue (Variables|Default|GetMainMenuRef) "DoNotLock")
  (Variables|/Script/Engine.PlayerController|SetbShowMouseCursor _returnvalue true))